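; Calibration camera that presents test color series on a canvas and post material, apparently for display color calibration.
; BeginPlay stencils the camera's child primitives through custom depth, creates the canvas's dynamic material, loads CSV plate points, spawns a Dots actor at the canvas and hides it.
; CalibrationPresentation selects primaries, stepped, cube or confusion-line colors and feeds them to UpdateMaterials.
; Separate events switch camera settings and toggle color mode.
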(event Custom|CalibrationPresentation
  (params (which :type String))
  (switch string which
    (:Primaries
      (bind _returnvalue (Class|CalibratedCamera|PrimariesSerially))
      (CallFunction|UpdateMaterials _returnvalue))
    (:Stepped
      (bind _returnvalue_2 (Class|CalibratedCamera|SteppedPrimariesSerially))
      (CallFunction|UpdateMaterials _returnvalue_2))
    (:Cubed_small
      (bind _returnvalue_3 (Class|CalibratedCamera|CubeColorsSerially 0.4 0.6))
      (CallFunction|UpdateMaterials _returnvalue_3))
    (:Cubed_big
      (bind _returnvalue_4 (Class|CalibratedCamera|CubeColorsSerially 0.2 0.8))
      (CallFunction|UpdateMaterials _returnvalue_4))
    (:Confusion
      (bind _returnvalue_5 (Class|CalibratedCamera|ConfusionLinesSerially))
      (CallFunction|UpdateMaterials _returnvalue_5))))

(event Custom|ColorDisplay
  (Utilities|FlowControl|FlipFlop
    (:A
      (Class|CalibratedCamera|ColorModeon 1.0))
    (:B
      (Class|CalibratedCamera|ColorModeon 0.0))))

(event Custom|Switch
  (Class|CalibratedCamera|SwitchCameraSettings))

(event EventBeginPlay
  (bind _canvas (Variables|Default|GetCanvas))
  (for _array_element (Components|GetChildrenComponents (Variables|Default|GetCameraComponent) false)
    (bind _asprimitive_component (Utilities|Casting|CastToPrimitiveComponent _array_element))
    (Rendering|SetRenderCustomDepth _asprimitive_component true)
    (Rendering|SetCustomDepthStencilValue _asprimitive_component 5))
  (bind _returnvalue (Rendering|Material|CreateDynamicMaterialInstance "/Game/Canvas_material.Canvas_material" "None" "None" :!class /Script/Engine.KismetMaterialLibrary))
  (bind _output_get (Variables|Default|Setcanvas_mat _returnvalue))
  (Rendering|Material|SetMaterial _canvas 0 _output_get)
  (bind _returnvalue_2 (Game|ConstructObjectfromClass "/Script/ColorCalibration.ColorCalibration" _canvas))
  (Utilities|FlowControl|Sequence
    (:then_1
      (bind _all_plates (Class|ColorCalibration|ReadPlatePointsfromCSV _returnvalue_2 "points.csv"))
      (bind _returnvalue_3 (Game|SpawnActorfromClass "/Game/dots.dots_C" (Math|Transform|MakeTransform (Transformation|GetWorldLocation _canvas) (Transformation|GetWorldRotation _canvas) "100.000000,100.000000,100.000000") "Undefined" 0 0))
      (Rendering|SetVisibility (Variables|Default|GetCanvas) false false)
      (Development|PrintString (Utilities|String|ToString(Vector) (Transformation|GetActorLocation _returnvalue_3)) true true "(R=0.000000,G=0.660000,B=1.000000,A=1.000000)" 1e+02))))

(event Collision|EventActorBeginOverlap
  (params (OtherActor :type Actor%20Object%20Reference)))

(event EventTick
  (params (DeltaSeconds :type Float%20%28single-precision%29)))

(fn ConstructionScript)

(fn UpdateMaterials
  (params (Input :type Linear%20Color%20Structure))
  (bind _canvas_mat (Variables|Default|Getcanvas_mat))
  (Class|CalibratedCamera|UpdatePostMaterial Input)
  (Rendering|Material|SetVectorParameterValue _canvas_mat "Color" Input :!class /Script/Engine.MaterialInstanceDynamic)
  (Rendering|Material|SetMaterial (Variables|Default|GetCanvas) 0 _canvas_mat))